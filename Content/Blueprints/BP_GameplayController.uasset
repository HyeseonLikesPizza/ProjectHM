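; BP_GameplayController is a gameplay controller Blueprint that manages the player's inventory screen.
; The Inventory input creates WB_Inventory and adds it to the viewport on first press, then toggles its visibility on later presses, switching mouse cursor and input mode with it.
; A ReloadInventory event calls LoadInventory on the existing widget, and leftover disconnected nodes never run.
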(event EventBeginPlay)

(event EventTick
  (params (DeltaSeconds :type Float%20%28single-precision%29)))

(event EventReloadInventory
  (bind _inventorywidget (Variables|Default|GetInventoryWidget))
  (Utilities|IsValid _inventorywidget
    (:Is%20Valid
      (Default|LoadInventory (.AsWB%20Inventory (Utilities|Casting|CastToWB_Inventory _inventorywidget))))))

(event Input|ActionEvents|InputActionInventory
  (params (Key :type Key%20Structure :default "None"))
  (bind _returnvalue (Game|GetPlayerController 0))
  (:Pressed
    (bind _inventorywidget (Variables|Default|GetInventoryWidget)
      (:then
        (if (Variables|Default|GetInventoryWidgetVisibility)
          (Widget|SetVisibility (Variables|Default|GetInventoryWidget) "Hidden")
          (Variables|Default|SetInventoryWidgetVisibility false)
          (Variables|/Script/Engine.PlayerController|SetbShowMouseCursor _returnvalue false)
          (Input|SetInputModeGameOnly _returnvalue)
          (else
            (Widget|SetVisibility (Variables|Default|GetInventoryWidget) "Visible")
            (Variables|Default|SetInventoryWidgetVisibility true)
            (Variables|/Script/Engine.PlayerController|SetbShowMouseCursor _returnvalue true)
            (Input|SetInputModeGameandUI _returnvalue (Variables|Default|GetInventoryWidget) "DoNotLock" true))))
      (:else
        (bind _returnvalue_2 (UserInterface|CreateWidget "/Game/UI/WB_Inventory.WB_Inventory_C" (Game|GetPlayerController 0)))
        (bind _output_get (Variables|Default|SetInventoryWidget _returnvalue_2))
        (UserInterface|Viewport|AddtoViewport _output_get 0)))))

(fn ConstructionScript)